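; StarbaseMesh is a mesh actor that resolves its static mesh and thumbnail render target from its own class name.
; The construction script optionally loads the matching mesh from BP_Meshes/Meshes, using the class name minus its two-character suffix.
; It can also add a scene capture framed diagonally from the mesh bounds, targeting the like-named render target in BP_Meshes/Thumbnails.
; CaptureThumbnail triggers that capture on demand.
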(event `Capture Thumbnail`
  (bind _thumbnailcamera (`self.ThumbnailCamera`)
    (:`then`
      (`SceneCaptureComponent2D.CaptureScene` _thumbnailcamera)
      (`KismetSystemLibrary.PrintString` "Scene Captured"))
    (:`else`)))

(fn `Get Asset Name`
  (returns (ReturnValue :type String))
  (return (`KismetStringLibrary.LeftChop` (`KismetSystemLibrary.GetClassDisplayName` (`GameplayStatics.GetObjectClass` self)) 2)))

(fn `UserConstructionScript`
  (bind (_origin _boxextent _sphereradius) (`KismetSystemLibrary.GetComponentBounds` (`self.StaticMeshComponent`)))
  (bind _returnvalue (+ _origin (`KismetMathLibrary.MakeVector` 0.0 0.0 (* _sphereradius 0.1))))
  (bind _returnvalue_2 (+ (* (0.5 0.5 0.5) (* _sphereradius 3.0)) _returnvalue))
  (`|ExecutionSequence`
    (:`then_0`
      (if (`self.Auto Apply Mesh`)
        (bind (_isvalid _returnvalue_3) (`VictoryBPFunctionLibrary.LoadObjectFromAssetPath` "/Script/Engine.StaticMesh" (`KismetStringLibrary.Conv_StringToName` (`VictoryBPFunctionLibrary.AppendMultiple` "/Game/BP_Meshes/Meshes/" (`self.Get Asset Name`)))))
        (if _isvalid
          (bind _asstatic_mesh (cast `StaticMesh` _returnvalue_3))
          (`StaticMeshComponent.SetStaticMesh` (`self.StaticMeshComponent`) _asstatic_mesh))))
    (:`then_1`
      (if (`self.Thumbnail Camera`)
        (bind _returnvalue_4 (`AddComponent|NODE_AddSceneCaptureComponent2D-0`))
        (bind _output_get (set `self.ThumbnailCamera` _returnvalue_4))
        (`SceneComponent.K2_SetWorldLocationAndRotation` _output_get _returnvalue_2 (`KismetMathLibrary.FindLookAtRotation` _returnvalue_2 _returnvalue) false false)
        (set `SceneCaptureComponent.MaxViewDistanceOverride` (* (`.SphereRadius` (`KismetSystemLibrary.GetComponentBounds` (`self.StaticMeshComponent`))) 4.0) (`self.ThumbnailCamera`))
        (bind (_isvalid_2 _returnvalue_5) (`VictoryBPFunctionLibrary.LoadObjectFromAssetPath` "/Script/Engine.TextureRenderTarget2D" (`KismetStringLibrary.Conv_StringToName` (`VictoryBPFunctionLibrary.AppendMultiple` "/Game/BP_Meshes/Thumbnails/" (`self.Get Asset Name`)))))
        (bind _astexture_render_target_2d (cast `TextureRenderTarget2D` _returnvalue_5))
        (set `SceneCaptureComponent2D.TextureTarget` _astexture_render_target_2d (`self.ThumbnailCamera`))))))