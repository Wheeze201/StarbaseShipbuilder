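; HUD Blueprint that owns the spawn menu widget and controls when it is shown.
; On BeginPlay it creates the SpawnMenu widget and adds it to the viewport.
; ShowSpawnMenu toggles the widget between visible and collapsed, along with player 0's mouse cursor.
; It also switches input between Game and UI, focused on the menu, and Game Only.
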(event `self.ReceiveBeginPlay`
  (`self.Create Widgets`))

(event `Create Widgets`
  (`|ExecutionSequence`
    (:`then_0`
      (bind _returnvalue (`|CreateWidget` "/Game/UI/SpawnMenu.SpawnMenu_C"))
      (set `self.SpawnMenu` _returnvalue))
    (:`then_1`
      (`UserWidget.AddToViewport` (`self.SpawnMenu`) 0))))

(fn `Show Spawn Menu`
  (params (Bool :type Boolean))
  (`Widget.SetVisibility` (`self.SpawnMenu`) (select `bool` Bool :`false` "Collapsed" :`true` "Visible" :!type "ESlateVisibility Enum"))
  (set `PlayerController.bShowMouseCursor` (`local.Bool`) (`GameplayStatics.GetPlayerController` 0))
  (if (`local.Bool`)
    (`WidgetBlueprintLibrary.SetInputMode_GameAndUIEx` (`GameplayStatics.GetPlayerController` 0) (`self.SpawnMenu`))
    (else
      (`WidgetBlueprintLibrary.SetInputMode_GameOnly` (`GameplayStatics.GetPlayerController` 0)))))

(fn `UserConstructionScript`)